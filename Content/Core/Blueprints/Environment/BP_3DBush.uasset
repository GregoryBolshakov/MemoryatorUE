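; BP_3DBush is an environment bush that varies its look by random variant and by biome.
; RandomizeAppearanceID picks one of five appearance IDs, and ApplyAppearanceID maps it to a bush mesh and matching BB material in slot 2.
; All variants then share a biome switch that sets the leaf material in slot 1 for Dark Woods, Birch Grove or Swamp.
; Branches for a sixth and seventh mesh exist but never run.
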(event EventRandomizeAppearanceID
  (Class|MActor|SetAppearanceID (Math|Random|RandomInteger 5)))

(event EventApplyAppearanceID
  (bind _staticmesh (Variables|Default|GetStaticMesh))
  (switch int (Variables|Default|GetAppearanceID)
    (:0
      (Components|StaticMesh|SetStaticMesh _staticmesh "/Game/DreamscapeSeries/DreamscapeTower/Meshes/Foliage/SM_Bush_01_WIP.SM_Bush_01_WIP")
      (Rendering|Material|SetMaterial _staticmesh 2 "/Game/Core/Environment/Vegetation/Trees/Dreamscape/Materials/MI_TreeA_01_BB.MI_TreeA_01_BB"))
    (:1
      (Components|StaticMesh|SetStaticMesh _staticmesh "/Game/DreamscapeSeries/DreamscapeTower/Meshes/Foliage/SM_Bush_02_WIP.SM_Bush_02_WIP")
      (Rendering|Material|SetMaterial _staticmesh 2 "/Game/Core/Environment/Vegetation/Trees/Dreamscape/Materials/MI_TreeA_02_BB.MI_TreeA_02_BB"))
    (:2
      (Components|StaticMesh|SetStaticMesh _staticmesh "/Game/DreamscapeSeries/DreamscapeTower/Meshes/Foliage/SM_Bush_03_WIP.SM_Bush_03_WIP")
      (Rendering|Material|SetMaterial _staticmesh 2 "/Game/Core/Environment/Vegetation/Trees/Dreamscape/Materials/MI_TreeA_03_BB.MI_TreeA_03_BB"))
    (:3
      (Components|StaticMesh|SetStaticMesh _staticmesh "/Game/DreamscapeSeries/DreamscapeTower/Meshes/Foliage/SM_Bush_04_WIP.SM_Bush_04_WIP")
      (Rendering|Material|SetMaterial _staticmesh 2 "/Game/Core/Environment/Vegetation/Trees/Dreamscape/Materials/MI_TreeB_01_BB.MI_TreeB_01_BB"))
    (:4
      (Components|StaticMesh|SetStaticMesh _staticmesh "/Game/DreamscapeSeries/DreamscapeTower/Meshes/Foliage/SM_Bush_05_WIp.SM_Bush_05_WIP")
      (Rendering|Material|SetMaterial _staticmesh 2 "/Game/Core/Environment/Vegetation/Trees/Dreamscape/Materials/MI_TreeC_01_BB.MI_TreeC_01_BB")))
  (bind _returnvalue (Class|MActor|GetMyBiome))
  (switch Utilities|FlowControl|Switch|SwitchonEBiome _returnvalue
    (:DarkWoods
      (Rendering|Material|SetMaterial _staticmesh 1 "/Game/Core/Environment/Vegetation/Trees/Dreamscape/Materials/MI_TreeLeaves_DarkWoods.MI_TreeLeaves_DarkWoods"))
    (:BirchGrove
      (Rendering|Material|SetMaterial _staticmesh 1 "/Game/Core/Environment/Vegetation/Trees/Dreamscape/Materials/MI_TreeLeaves_BirchGrove.MI_TreeLeaves_BirchGrove"))
    (:Swamp
      (Rendering|Material|SetMaterial _staticmesh 1 "/Game/Core/Environment/Vegetation/Trees/Dreamscape/Materials/MI_TreeLeaves_Swamp.MI_TreeLeaves_Swamp"))))

(fn ConstructionScript)