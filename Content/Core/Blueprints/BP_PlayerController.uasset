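; Player controller that manages hero persistence, camera occlusion checks, the experience level HUD and floating XP numbers.
; On start it loads the local save, sends it through the Nakama UserManagerClient and requests the hero data back.
; A looping timer and Destroyed repeat that round trip, then save asynchronously after a short delay.
; MakeFloatingNumber spawns one Niagara system per character, offset sideways and textured with its digit or XP glyph.
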(event Custom|EventSave
  (bind _user_manager_client (Variables|Default|GetUser%20Manager%20Client))
  (bind _user_manager_client_2 (Variables|Default|GetUser%20Manager%20Client))
  (bind _hero (Variables|/Script/NakamaManager.UserManagerClient|GetHero _user_manager_client))
  ;[1 1 1 1 30] Setup autosaves
  ;;[1 1 1 1 28] Send to server -> (It validates) -> Update from server
  (EventDispatchers|AssignHeroDataSentDelegate _user_manager_client_2 (delegate Custom|HeroDataSentDelegate_Event2))
  (Class|UserManagerClient|SendHeroData _user_manager_client_2)
  (Utilities|FlowControl|Delay 1.0)
  ;;[1 1 1 1 30] Save to memory
  (bind _returnvalue (SaveGame|CreateSaveGameObject "/Game/Core/Blueprints/Saves/BP_SaveHero.BP_SaveHero_C"))
  (Variables|/Game/Core/Blueprints/Saves/BP_SaveHero.BP_SaveHero_C|SetName _returnvalue (.name _hero))
  (Variables|/Game/Core/Blueprints/Saves/BP_SaveHero.BP_SaveHero_C|SetLevel _returnvalue (.level _hero))
  (Variables|/Game/Core/Blueprints/Saves/BP_SaveHero.BP_SaveHero_C|SetExperience _returnvalue (.experience _hero))
  (|AsyncSaveGametoSlot self _returnvalue (Variables|Default|GetSaveSlotName)))

(event Custom|HeroDataSentDelegate_Event2
  (params (rpc :type Nakama%20RPC%20Structure%20%28by%20ref%29))
  ;[1 1 1 1 30] Setup autosaves
  ;;[1 1 1 1 28] Send to server -> (It validates) -> Update from server
  (Class|UserManagerClient|RequestHeroData (Variables|Default|GetUser%20Manager%20Client)))

(event Custom|Check%20Occluded%20By%20Camera
  ;[1 1 1] Set Occlusion Check Timer
  (Class|MPlayerController|SyncOccludedActors))

(event Custom|HeroDataSentDelegate_Event
  (params (rpc :type Nakama%20RPC%20Structure%20%28by%20ref%29))
  ;[1 1 1 1 24] Load from save -> Send to server -> (It validates) -> Update from server
  (Class|UserManagerClient|RequestHeroData (Variables|Default|GetUser%20Manager%20Client)))

(event EventBeginPlay
  ;[1 1 1] Set Occlusion Check Timer
  (Utilities|Time|SetTimerbyEvent (delegate Custom|Check%20Occluded%20By%20Camera) 0.1 true)
  ;[1 1 1 1 30] Set User Manager variable
  (bind _asmgame_instance (Utilities|Casting|CastToMGameInstance (Game|GetGameInstance)))
  (bind _returnvalue (Class|MGameInstance|GetNakamaManager _asmgame_instance))
  (Variables|Default|SetUser%20Manager%20Client (Variables|/Script/NakamaManager.NakamaManager|GetUserManagerClient _returnvalue))
  ;[1 1 1 1 24] Load from save -> Send to server -> (It validates) -> Update from server
  (CallFunction|LoadfromMemory)
  (EventDispatchers|AssignHeroDataSentDelegate (Variables|Default|GetUser%20Manager%20Client) (delegate Custom|HeroDataSentDelegate_Event))
  (Class|UserManagerClient|SendHeroData (Variables|Default|GetUser%20Manager%20Client))
  ;[1 1 1 1 30] Setup autosaves
  (Utilities|Time|SetTimerbyEvent (delegate Custom|EventSave) 5.0 true)
  ;[1 1 1 1 30] Create exp level widget
  (bind _returnvalue_2 (UserInterface|CreateWidget "/Game/Core/Widgets/WBP_ExperienceLevel.WBP_ExperienceLevel_C"))
  (UserInterface|Viewport|AddtoViewport _returnvalue_2 0))

(event EventDestroyed
  (CallFunction|EventSave))

(fn ConstructionScript)

(fn MakeFloatingNumber
  (params (Location :type Vector%20%28by%20ref%29 :default "0, 0, 0") (Value :type Integer) (Type :type EFloatingNumberType%20Enum :default "Experience"))
  (for _array_element (Utilities|String|GetCharacterArrayfromString (Utilities|String|Append (Utilities|String|ToString(Integer) Value) "X"))
    (bind _returnvalue (Niagara|SpawnSystematLocation "/Game/Core/Niagara/FloatingNumbersFX.FloatingNumbersFX" Location (Math|Rotator|MakeRotator 0.0 1.8e+02 (.yaw (Pawn|GetControlRotation (Game|GetPlayerController 0) :!class /Script/Engine.Controller)))))
    (bind _output_get (Variables|Default|SetDigitSystem _returnvalue))
    (Transformation|AddLocalOffset _output_get (Math|Vector|MakeVector 0.0 (Variables|Default|GetDigitTextOffset) 0.0) false false)
    (Variables|Default|SetDigitTextOffset (+ (Variables|Default|GetDigitTextOffset) 15.0))
    (switch string _array_element
      (:0
        (Niagara|SetTextureObject (Variables|Default|GetDigitSystem) "user.Digit" "/Game/Core/UI/Textures/NiagaraTextures/0.0"))
      (:1
        (Niagara|SetTextureObject (Variables|Default|GetDigitSystem) "user.Digit" "/Game/Core/UI/Textures/NiagaraTextures/1.1"))
      (:2
        (Niagara|SetTextureObject (Variables|Default|GetDigitSystem) "user.Digit" "/Game/Core/UI/Textures/NiagaraTextures/2.2"))
      (:3
        (Niagara|SetTextureObject (Variables|Default|GetDigitSystem) "user.Digit" "/Game/Core/UI/Textures/NiagaraTextures/3.3"))
      (:4
        (Niagara|SetTextureObject (Variables|Default|GetDigitSystem) "user.Digit" "/Game/Core/UI/Textures/NiagaraTextures/4.4"))
      (:5
        (Niagara|SetTextureObject (Variables|Default|GetDigitSystem) "user.Digit" "/Game/Core/UI/Textures/NiagaraTextures/5.5"))
      (:6
        (Niagara|SetTextureObject (Variables|Default|GetDigitSystem) "user.Digit" "/Game/Core/UI/Textures/NiagaraTextures/6.6"))
      (:7
        (Niagara|SetTextureObject (Variables|Default|GetDigitSystem) "user.Digit" "/Game/Core/UI/Textures/NiagaraTextures/7.7"))
      (:8
        (Niagara|SetTextureObject (Variables|Default|GetDigitSystem) "user.Digit" "/Game/Core/UI/Textures/NiagaraTextures/8.8"))
      (:9
        (Niagara|SetTextureObject (Variables|Default|GetDigitSystem) "user.Digit" "/Game/Core/UI/Textures/NiagaraTextures/9.9"))
      (:X
        (Niagara|SetTextureObject (Variables|Default|GetDigitSystem) "user.Digit" "/Game/Core/UI/Textures/NiagaraTextures/xp.xp"))))
  (Variables|Default|SetDigitTextOffset 0.0))

(fn LoadfromMemory
  (bind _returnvalue (SaveGame|LoadGamefromSlot (Variables|Default|GetSaveSlotName)))
  (bind _asbp_save_hero (Utilities|Casting|CastToBP_SaveHero _returnvalue)
    (:then
      (Variables|/Script/NakamaManager.UserManagerClient|SetHero (Variables|Default|GetUser%20Manager%20Client) (Utilities|Struct|MakeHero (Variables|/Game/Core/Blueprints/Saves/BP_SaveHero.BP_SaveHero_C|GetName _asbp_save_hero) (Variables|/Game/Core/Blueprints/Saves/BP_SaveHero.BP_SaveHero_C|GetLevel _asbp_save_hero) (Variables|/Game/Core/Blueprints/Saves/BP_SaveHero.BP_SaveHero_C|GetExperience _asbp_save_hero))))
    (:CastFailed
      (Utilities|String|LogString "BP_PlayerController: Couldn't load save"))))