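; BP_PCG_RandomChoice is a custom PCG Blueprint element, apparently meant to randomly keep a subset of points, but it is unfinished.
; ExecuteWithContext returns immediately without producing output.
; Disconnected logic reads point data from the "In" pin and computes a keep count from either a clamped fixed number or a rounded-up ratio.
; No random selection or output writing is implemented.
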(fn ExecutewithContext
  (params (InContext :type PCG%20Context%20Structure%20%28by%20ref%29) (Input :type PCG%20Data%20Collection%20Structure%20%28by%20ref%29))
  (return ""))