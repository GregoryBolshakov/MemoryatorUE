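; BP_NightmareMedium is a medium nightmare mob pawn that drives its body flipbook animation and reports combat timing to its MMobController.
; On possession it caches the controller.
; UpdateAnimation restarts the flipbook and picks Move, Fight or Idle from the movement and fighting flags.
; During Fight, flipbook delegates notify the controller when the animation ends and register a hit on a specific sprite frame.
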(event Custom|OnSpriteChanged
  ;[1 1 1] Fight animation
  ;;[1 1 1] Bind the striking sprite of the animation with controller
  (if (== (Class|PaperFlipbookComponent|GetPlaybackPositioninFrames (Variables|Default|GetFlipbookBody)) 5)
    (Class|MMobController|OnHit (Variables|Default|GetMobController))))

(event Custom|OnFightAnimationEnd
  ;[1 1 1] Fight animation
  ;;[1 1 1] Bind the end of the fight animation with controller
  (Class|MInterfaceMobController|OnFightAnimationEnd (Variables|Default|GetMobController)))

(event EventUpdateAnimation
  (bind _flipbookbody (Variables|Default|GetFlipbookBody))
  ;[1 1 1] Reset all bindings and play flipbook from start
  (EventDispatchers|UnbindallEventsfromOnFinishedPlaying _flipbookbody)
  (Components|Timeline|PlayfromStart _flipbookbody)
  (if (Variables|Default|GetIsMoving)
    ;[1 1 1] Move animation
    (Class|MRotatableFlipbookComponent|SetAction (Variables|Default|GetFlipbookBody) (Utilities|Name|MakeLiteralName "Move"))
    (elif (Variables|Default|GetIsFighting)
      ;[1 1 1] Fight animation
      (Class|MRotatableFlipbookComponent|SetAction (Variables|Default|GetFlipbookBody) (Utilities|Name|MakeLiteralName "Fight"))
      ;;[1 1 1] Bind the end of the fight animation with controller
      (EventDispatchers|BindEventtoOnFinishedPlaying (Variables|Default|GetFlipbookBody) (delegate Custom|OnFightAnimationEnd))
      ;;[1 1 1] Bind the striking sprite of the animation with controller
      (EventDispatchers|BindEventtoOnSpriteChangeDelegate (Variables|Default|GetFlipbookBody) (delegate Custom|OnSpriteChanged))
      (else
        ;[1 1 1] Idle animation
        (Class|MRotatableFlipbookComponent|SetAction (Variables|Default|GetFlipbookBody) (Utilities|Name|MakeLiteralName "Idle"))))))

(event EventPossessed
  (params (NewController :type Controller%20Object%20Reference))
  (bind _asmmob_controller (Utilities|Casting|CastToMMobController (Pawn|GetController)))
  (Variables|Default|SetMobController _asmmob_controller))

(fn ConstructionScript)