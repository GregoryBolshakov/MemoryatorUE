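; Test tree actor that takes a random sprite to match the biome it is given.
; The Randomize event branches on DarkWoods, BirchGrove or Swamp and sets SpriteTree to a random pick from that biome's sprites.
; DarkWoods lists its first sprite twice, making it more likely, and any other biome draws a red "No biome specified" debug message.
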(event EventRandomize
  (params (Biome :type EBiome%20Enum :default "DarkWoods"))
  (bind _spritetree (Variables|Default|GetSpriteTree))
  (bind _spritetree_2 (Variables|Default|GetSpriteTree))
  (bind _spritetree_3 (Variables|Default|GetSpriteTree))
  (if (Utilities|Enum|Equal(Enum) Biome "DarkWoods")
    (switch int (Math|Random|RandomInteger 6)
      (:0
        (Rendering|Components|Sprite|SetSprite _spritetree_2 "/Game/Memoryator/Textures/World/DarkWoods/Frames/DarkWoods_tree_1_png.DarkWoods_tree_1_png"))
      (:1
        (Rendering|Components|Sprite|SetSprite _spritetree_2 "/Game/Memoryator/Textures/World/DarkWoods/Frames/DarkWoods_tree_2_png.DarkWoods_tree_2_png"))
      (:2
        (Rendering|Components|Sprite|SetSprite _spritetree_2 "/Game/Memoryator/Textures/World/DarkWoods/Frames/DarkWoods_tree_3_png.DarkWoods_tree_3_png"))
      (:3
        (Rendering|Components|Sprite|SetSprite _spritetree_2 "/Game/Memoryator/Textures/World/DarkWoods/Frames/DarkWoods_tree_4_png.DarkWoods_tree_4_png"))
      (:4
        (Rendering|Components|Sprite|SetSprite _spritetree_2 "/Game/Memoryator/Textures/World/DarkWoods/Frames/DarkWoods_tree_1_png.DarkWoods_tree_1_png"))
      (:5
        (Rendering|Components|Sprite|SetSprite _spritetree_2 "/Game/Memoryator/Textures/World/DarkWoods/Frames/DarkWoods_tree_5_png.DarkWoods_tree_5_png")))
    (elif (Utilities|Enum|Equal(Enum) Biome "BirchGrove")
      (switch int (Math|Random|RandomInteger 7)
        (:0
          (Rendering|Components|Sprite|SetSprite _spritetree_3 "/Game/Memoryator/Textures/World/BirchGrove/Frames/tree_1_png.tree_1_png"))
        (:1
          (Rendering|Components|Sprite|SetSprite _spritetree_3 "/Game/Memoryator/Textures/World/BirchGrove/Frames/tree_2_png.tree_2_png"))
        (:2
          (Rendering|Components|Sprite|SetSprite _spritetree_3 "/Game/Memoryator/Textures/World/BirchGrove/Frames/tree_3_png.tree_3_png"))
        (:3
          (Rendering|Components|Sprite|SetSprite _spritetree_3 "/Game/Memoryator/Textures/World/BirchGrove/Frames/tree_4_png.tree_4_png"))
        (:4
          (Rendering|Components|Sprite|SetSprite _spritetree_3 "/Game/Memoryator/Textures/World/BirchGrove/Frames/tree_5_png.tree_5_png"))
        (:5
          (Rendering|Components|Sprite|SetSprite _spritetree_3 "/Game/Memoryator/Textures/World/BirchGrove/Frames/tree_6_png.tree_6_png"))
        (:6
          (Rendering|Components|Sprite|SetSprite _spritetree_3 "/Game/Memoryator/Textures/World/BirchGrove/Frames/tree_7_png.tree_7_png")))
      (elif (Utilities|Enum|Equal(Enum) Biome "Swamp")
        (switch int (Math|Random|RandomInteger 5)
          (:0
            (Rendering|Components|Sprite|SetSprite _spritetree "/Game/Memoryator/Textures/World/Swamp/Frames/SwampyTrees_tree_1_png.SwampyTrees_tree_1_png"))
          (:1
            (Rendering|Components|Sprite|SetSprite _spritetree "/Game/Memoryator/Textures/World/Swamp/Frames/SwampyTrees_tree_2_png.SwampyTrees_tree_2_png"))
          (:2
            (Rendering|Components|Sprite|SetSprite _spritetree "/Game/Memoryator/Textures/World/Swamp/Frames/SwampyTrees_tree_3_png.SwampyTrees_tree_3_png"))
          (:3
            (Rendering|Components|Sprite|SetSprite _spritetree "/Game/Memoryator/Textures/World/Swamp/Frames/SwampyTrees_tree_4_png.SwampyTrees_tree_4_png"))
          (:4
            (Rendering|Components|Sprite|SetSprite _spritetree "/Game/Memoryator/Textures/World/Swamp/Frames/SwampyTrees_tree_5_png.SwampyTrees_tree_5_png")))
        (else
          (Rendering|Debug|DrawDebugString "0, 0, 0" "No biome specified" 0 "(R=1.000000,G=0.000000,B=0.000000,A=1.000000)" 5.0))))))

(fn ConstructionScript)