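; Grass spawn area actor for DynamicGrassLite that builds a visible volume from a random geometry preset in its construction script.
; The preset's vertices and triangles form a procedural floor mesh with collision, and a copy raised by the area height forms the ceiling.
; Thin instanced pillars at each vertex show the height, and both mesh sections use a simple translucent material.
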(fn ConstructionScript
  (bind _proceduralmesh_0 (Variables|Default|GetProceduralMesh_0))
  (bind _proceduralmesh_0_2 (Variables|Default|GetProceduralMesh_0))
  ;[1 1 1] Get random geometry preset
  (bind _output_get (Variables|Default|SetGeometryPreset_0 (.OutItem (Utilities|Array|Random (Variables|/Script/TopDownTemp.GrassSpawnAreaGeometryDataAsset|GetPresets (Variables|Default|GetGeometryDataAsset_0))))))
  (Variables|Default|SetV_0 (.v _output_get))
  (Variables|Default|Settriangles_0 (.triangles _output_get))
  (Variables|Default|SetareaHeight_0 (.areaheight _output_get))
  (Variables|Default|SetV_Ceiling_0 (.v_celling _output_get))
  (if true
    (Class|ProceduralMeshComponent|CreateMeshSectionLinearColor _proceduralmesh_0_2 0 (Variables|Default|GetV_0) (Variables|Default|Gettriangles_0) 0 0 0 0 0 0 0 true false)
    (Rendering|Material|SetMaterial _proceduralmesh_0_2 0 "/Game/Memoryator/Blueprints/Environment/DynamicGrassLite/Materials/Misc/SimpleTranslucent_M.SimpleTranslucent_M")
    (Components|InstancedStaticMesh|ClearInstances (Variables|Default|GetHeightVisPillars_0))
    (Utilities|Array|Clear (Variables|Default|GetV_Ceiling_0))
    (for _array_element (Variables|Default|GetV_0)
      (Utilities|Array|Add (Variables|Default|GetV_Ceiling_0) (+ _array_element (Math|Vector|MakeVector 0.0 0.0 (Variables|Default|GetareaHeight_0))))
      (Components|InstancedStaticMesh|AddInstance (Variables|Default|GetHeightVisPillars_0) (Math|Transform|MakeTransform _array_element "0, 0, 0" (Math|Vector|MakeVector 0.01 0.01 (Variables|Default|GetareaHeight_0))) false))
    (Class|ProceduralMeshComponent|CreateMeshSectionLinearColor _proceduralmesh_0 1 (Variables|Default|GetV_Ceiling_0) (Variables|Default|Gettriangles_0) 0 0 0 0 0 0 0 false false)
    (Rendering|Material|SetMaterial _proceduralmesh_0 1 "/Game/Memoryator/Blueprints/Environment/DynamicGrassLite/Materials/Misc/SimpleTranslucent_M.SimpleTranslucent_M")
    (else
      (Utilities|String|LogString "Couldn't find geometry preset"))))