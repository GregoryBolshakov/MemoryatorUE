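; BP_Nightmare is the Blueprint for the Nightmare in Memoryator, handling its body flipbook animation.
; UpdateAnimation resets looping and finish bindings, restarts playback, then picks the Move, Fight or Idle action from IsMoving and IsFighting, with movement taking priority.
; The Fight action plays once and binds an event to its finish, while Move and Idle loop.
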(event EventUpdateAnimation
  (bind _bodyflipbook (Variables|Default|GetBodyFlipbook))
  (bind _bodyflipbook_2 (Variables|Default|GetBodyFlipbook))
  (Components|Timeline|SetLooping _bodyflipbook true)
  (EventDispatchers|UnbindallEventsfromOnFinishedPlaying _bodyflipbook)
  (Components|Timeline|PlayfromStart _bodyflipbook)
  (if (Variables|Default|GetIsMoving)
    (Class|MRotatableFlipbookComponent|SetAction (Variables|Default|GetBodyFlipbook) (Utilities|Name|MakeLiteralName "Move"))
    (elif (Variables|Default|GetIsFighting)
      (Class|MRotatableFlipbookComponent|SetAction _bodyflipbook_2 (Utilities|Name|MakeLiteralName "Fight"))
      (Components|Timeline|SetLooping _bodyflipbook_2 false)
      (EventDispatchers|BindEventtoOnFinishedPlaying _bodyflipbook_2 (EventDispatchers|CreateEvent :!event OnFightingAnimationFinished))
      (else
        (Class|MRotatableFlipbookComponent|SetAction (Variables|Default|GetBodyFlipbook) (Utilities|Name|MakeLiteralName "Idle"))))))

(fn ConstructionScript)