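; BP_3DTree is an environment tree whose look varies by appearance ID and biome.
; RandomizeAppearanceID picks one of five variants at random and stores it as the AppearanceID.
; ApplyAppearanceID sets that variant's static mesh and its BB material on slot 2, then sets the leaf material on slot 1 to match Dark Woods, Birch Grove or Swamp.
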(event EventRandomizeAppearanceID
  (Class|MActor|SetAppearanceID (Math|Random|RandomInteger 5)))

(event EventApplyAppearanceID
  (bind _staticmesh (Variables|Default|GetStaticMesh))
  (switch int (Variables|Default|GetAppearanceID)
    (:0
      (Components|StaticMesh|SetStaticMesh _staticmesh "/Game/DreamscapeSeries/DreamscapeTower/Meshes/Trees/SM_Tree_A_01.SM_Tree_A_01")
      (Rendering|Material|SetMaterial _staticmesh 2 "/Game/Memoryator/Materials/3DTrees/Billboard/MI_TreeA_01_BB.MI_TreeA_01_BB"))
    (:1
      (Components|StaticMesh|SetStaticMesh _staticmesh "/Game/DreamscapeSeries/DreamscapeTower/Meshes/Trees/SM_Tree_A_02.SM_Tree_A_02")
      (Rendering|Material|SetMaterial _staticmesh 2 "/Game/Memoryator/Materials/3DTrees/Billboard/MI_TreeA_02_BB.MI_TreeA_02_BB"))
    (:2
      (Components|StaticMesh|SetStaticMesh _staticmesh "/Game/DreamscapeSeries/DreamscapeTower/Meshes/Trees/SM_Tree_A_03.SM_Tree_A_03")
      (Rendering|Material|SetMaterial _staticmesh 2 "/Game/Memoryator/Materials/3DTrees/Billboard/MI_TreeA_03_BB.MI_TreeA_03_BB"))
    (:3
      (Components|StaticMesh|SetStaticMesh _staticmesh "/Game/DreamscapeSeries/DreamscapeTower/Meshes/Trees/SM_Tree_B_01.SM_Tree_B_01")
      (Rendering|Material|SetMaterial _staticmesh 2 "/Game/Memoryator/Materials/3DTrees/Billboard/MI_TreeB_01_BB.MI_TreeB_01_BB"))
    (:4
      (Components|StaticMesh|SetStaticMesh _staticmesh "/Game/DreamscapeSeries/DreamscapeTower/Meshes/Trees/SM_Tree_B_02.SM_Tree_B_02")
      (Rendering|Material|SetMaterial _staticmesh 2 "/Game/Memoryator/Materials/3DTrees/Billboard/MI_TreeC_01_BB.MI_TreeC_01_BB")))
  (bind _returnvalue (Class|MActor|GetMyBiome))
  (switch Utilities|FlowControl|Switch|SwitchonEBiome _returnvalue
    (:DarkWoods
      (Rendering|Material|SetMaterial _staticmesh 1 "/Game/Memoryator/Materials/3DTrees/Leaves/MI_TreeLeaves_DarkWoods.MI_TreeLeaves_DarkWoods"))
    (:BirchGrove
      (Rendering|Material|SetMaterial _staticmesh 1 "/Game/Memoryator/Materials/3DTrees/Leaves/MI_TreeLeaves_BirchGrove.MI_TreeLeaves_BirchGrove"))
    (:Swamp
      (Rendering|Material|SetMaterial _staticmesh 1 "/Game/Memoryator/Materials/3DTrees/Leaves/MI_TreeLeaves_Swamp.MI_TreeLeaves_Swamp"))))

(fn ConstructionScript)