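; Character Blueprint that animates a character built from separate body and legs flipbooks.
; An UpdateAnimation event reads the IsMoving flag and sets both flipbooks to either the Move or Idle action together.
; The construction script is empty, and nothing here sets IsMoving or triggers the update.
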(event EventUpdateAnimation
  (if (Variables|Default|GetIsMoving)
    (Class|MRotatableFlipbookComponent|SetAction (Variables|Default|GetBodyFlipbook) (Utilities|Name|MakeLiteralName "Move"))
    (Class|MRotatableFlipbookComponent|SetAction (Variables|Default|GetLegsFlipbook) (Utilities|Name|MakeLiteralName "Move"))
    (else
      (Class|MRotatableFlipbookComponent|SetAction (Variables|Default|GetBodyFlipbook) (Utilities|Name|MakeLiteralName "Idle"))
      (Class|MRotatableFlipbookComponent|SetAction (Variables|Default|GetLegsFlipbook) (Utilities|Name|MakeLiteralName "Idle")))))

(fn ConstructionScript)