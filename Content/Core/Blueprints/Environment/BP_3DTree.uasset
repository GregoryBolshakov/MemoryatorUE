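; BP_3DTree is an environment tree actor whose look depends on the biome it belongs to.
; RandomizeAppearanceID rolls an AppearanceID within the variant count for the current biome.
; ApplyAppearanceID maps that ID to a spruce (Dark Woods), birch (Birch Grove) or pine (Swamp) mesh and sets that species' bark and foliage materials.
; An obsolete, unconnected branch still references older tree meshes with billboard materials.
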(event EventRandomizeAppearanceID
  (bind _returnvalue (Class|MActor|GetMyBiome))
  (switch Utilities|FlowControl|Switch|SwitchonEBiome _returnvalue
    (:DarkWoods
      (Class|MActor|SetAppearanceID (Math|Random|RandomInteger 6)))
    (:BirchGrove
      (Class|MActor|SetAppearanceID (Math|Random|RandomInteger 8)))
    (:Swamp
      (Class|MActor|SetAppearanceID (Math|Random|RandomInteger 8)))))

(event EventApplyAppearanceID
  (bind _staticmesh (Variables|Default|GetStaticMesh))
  (bind _staticmesh_2 (Variables|Default|GetStaticMesh))
  (bind _staticmesh_3 (Variables|Default|GetStaticMesh))
  (bind _returnvalue (Class|MActor|GetMyBiome))
  (switch Utilities|FlowControl|Switch|SwitchonEBiome _returnvalue
    (:DarkWoods
      ;[1 1 1] Dark Woods
      (switch int (Variables|Default|GetAppearanceID)
        (:0
          (Components|StaticMesh|SetStaticMesh _staticmesh_3 "/Game/Core/Environment/Vegetation/Trees/Slavic/Meshes/SM_sf2_spruce_01.SM_sf2_spruce_01"))
        (:1
          (Components|StaticMesh|SetStaticMesh _staticmesh_3 "/Game/Core/Environment/Vegetation/Trees/Slavic/Meshes/SM_sf2_spruce_02.SM_sf2_spruce_02"))
        (:2
          (Components|StaticMesh|SetStaticMesh _staticmesh_3 "/Game/Core/Environment/Vegetation/Trees/Slavic/Meshes/SM_sf2_spruce_03.SM_sf2_spruce_03"))
        (:3
          (Components|StaticMesh|SetStaticMesh _staticmesh_3 "/Game/Core/Environment/Vegetation/Trees/Slavic/Meshes/SM_sf2_spruce_04.SM_sf2_spruce_04"))
        (:4
          (Components|StaticMesh|SetStaticMesh _staticmesh_3 "/Game/Core/Environment/Vegetation/Trees/Slavic/Meshes/SM_sf2_spruce_05.SM_sf2_spruce_05"))
        (:5
          (Components|StaticMesh|SetStaticMesh _staticmesh_3 "/Game/Core/Environment/Vegetation/Trees/Slavic/Meshes/SM_sf2_spruce_06.SM_sf2_spruce_06")))
      (Rendering|Material|SetMaterial _staticmesh_3 1 "/Game/Core/Environment/Vegetation/Trees/Slavic/Materials/ByBiomes/DarkWoods/MI_sf2_spruce_foliage_Inst.MI_sf2_spruce_foliage_Inst")
      (Rendering|Material|SetMaterial _staticmesh_3 0 "/Game/Core/Environment/Vegetation/Trees/Slavic/Materials/ByBiomes/DarkWoods/MI_sf2_spruce_bark_Inst.MI_sf2_spruce_bark_Inst"))
    (:BirchGrove
      ;[1 1 1] Birch Grove
      (switch int (Variables|Default|GetAppearanceID)
        (:0
          (Components|StaticMesh|SetStaticMesh _staticmesh "/Game/Core/Environment/Vegetation/Trees/Slavic/Meshes/SM_sf2_birch_01.SM_sf2_birch_01"))
        (:1
          (Components|StaticMesh|SetStaticMesh _staticmesh "/Game/Core/Environment/Vegetation/Trees/Slavic/Meshes/SM_sf2_birch_02.SM_sf2_birch_02"))
        (:2
          (Components|StaticMesh|SetStaticMesh _staticmesh "/Game/Core/Environment/Vegetation/Trees/Slavic/Meshes/SM_sf2_birch_03.SM_sf2_birch_03"))
        (:3
          (Components|StaticMesh|SetStaticMesh _staticmesh "/Game/Core/Environment/Vegetation/Trees/Slavic/Meshes/SM_sf2_birch_04.SM_sf2_birch_04"))
        (:4
          (Components|StaticMesh|SetStaticMesh _staticmesh "/Game/Core/Environment/Vegetation/Trees/Slavic/Meshes/SM_sf2_birch_05.SM_sf2_birch_05"))
        (:5
          (Components|StaticMesh|SetStaticMesh _staticmesh "/Game/Core/Environment/Vegetation/Trees/Slavic/Meshes/SM_sf2_birch_06.SM_sf2_birch_06"))
        (:6
          (Components|StaticMesh|SetStaticMesh _staticmesh "/Game/Core/Environment/Vegetation/Trees/Slavic/Meshes/SM_sf2_birch_07.SM_sf2_birch_07"))
        (:7
          (Components|StaticMesh|SetStaticMesh _staticmesh "/Game/Core/Environment/Vegetation/Trees/Slavic/Meshes/SM_sf2_birch_08.SM_sf2_birch_08")))
      (Rendering|Material|SetMaterial _staticmesh 1 "/Game/Core/Environment/Vegetation/Trees/Slavic/Materials/ByBiomes/BirchGrove/MI_sf2_Birch_foliage_Inst.MI_sf2_Birch_foliage_Inst")
      (Rendering|Material|SetMaterial _staticmesh 0 "/Game/Core/Environment/Vegetation/Trees/Slavic/Materials/ByBiomes/BirchGrove/MI_sf2_birch_bark_Inst.MI_sf2_birch_bark_Inst"))
    (:Swamp
      ;[1 1 1] Birch Grove
      (switch int (Variables|Default|GetAppearanceID)
        (:0
          (Components|StaticMesh|SetStaticMesh _staticmesh_2 "/Game/Core/Environment/Vegetation/Trees/Slavic/Meshes/SM_sf2_pine_01.SM_sf2_pine_01"))
        (:1
          (Components|StaticMesh|SetStaticMesh _staticmesh_2 "/Game/Core/Environment/Vegetation/Trees/Slavic/Meshes/SM_sf2_pine_02.SM_sf2_pine_02"))
        (:2
          (Components|StaticMesh|SetStaticMesh _staticmesh_2 "/Game/Core/Environment/Vegetation/Trees/Slavic/Meshes/SM_sf2_pine_03.SM_sf2_pine_03"))
        (:3
          (Components|StaticMesh|SetStaticMesh _staticmesh_2 "/Game/Core/Environment/Vegetation/Trees/Slavic/Meshes/SM_sf2_pine_04.SM_sf2_pine_04"))
        (:4
          (Components|StaticMesh|SetStaticMesh _staticmesh_2 "/Game/Core/Environment/Vegetation/Trees/Slavic/Meshes/SM_sf2_pine_05.SM_sf2_pine_05"))
        (:5
          (Components|StaticMesh|SetStaticMesh _staticmesh_2 "/Game/Core/Environment/Vegetation/Trees/Slavic/Meshes/SM_sf2_pine_06.SM_sf2_pine_06"))
        (:6
          (Components|StaticMesh|SetStaticMesh _staticmesh_2 "/Game/Core/Environment/Vegetation/Trees/Slavic/Meshes/SM_sf2_pine_07.SM_sf2_pine_07"))
        (:7
          (Components|StaticMesh|SetStaticMesh _staticmesh_2 "/Game/Core/Environment/Vegetation/Trees/Slavic/Meshes/SM_sf2_pine_08.SM_sf2_pine_08")))
      (Rendering|Material|SetMaterial _staticmesh_2 1 "/Game/Core/Environment/Vegetation/Trees/Slavic/Materials/ByBiomes/Swamp/MI_sf2_PIne_foliage_Inst.MI_sf2_PIne_foliage_Inst")
      (Rendering|Material|SetMaterial _staticmesh_2 0 "/Game/Core/Environment/Vegetation/Trees/Slavic/Materials/ByBiomes/Swamp/MI_sf2_pine_bark_Inst.MI_sf2_pine_bark_Inst"))))

(fn ConstructionScript)