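; BP_Poppy is a pickable poppy environment flower with a small inventory.
; On BeginPlay it initialises that inventory with a random, small quantity of a single item type.
; A separate Randomize event picks one of three poppy sprites for the pickable item's sprite component, varying the flower's look.
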(event EventRandomize
  (params (Biome :type EBiome%20Enum :default "DarkWoods"))
  (bind _spritepickableiem (Variables|Default|GetSpritePickableIem))
  (switch int (Math|Random|RandomInteger 3)
    (:0
      (Rendering|Components|Sprite|SetSprite _spritepickableiem "/Game/Memoryator/Textures/Environment/Flowers/Frames/flowers_poppy_1_png.flowers_poppy_1_png"))
    (:1
      (Rendering|Components|Sprite|SetSprite _spritepickableiem "/Game/Memoryator/Textures/Environment/Flowers/Frames/flowers_poppy_2_png.flowers_poppy_2_png"))
    (:2
      (Rendering|Components|Sprite|SetSprite _spritepickableiem "/Game/Memoryator/Textures/Environment/Flowers/Frames/flowers_poppy_3_png.flowers_poppy_3_png"))))

(event EventBeginPlay
  (Class|MPickableActor|InitialiseInventory (Utilities|Array|MakeArray (Utilities|Struct|MakeItem 4 (Math|Random|RandomIntegerinRange 1 3)))))

(fn ConstructionScript)