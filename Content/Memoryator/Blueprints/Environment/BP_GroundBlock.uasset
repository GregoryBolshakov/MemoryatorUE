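; Ground block for the environment that restyles itself to match its biome: Dark Woods, Birch Grove or Swamp.
; On OnBiomeUpdated, it switches on GetMyBiome to set the grass material, the ground material and a shared transition material on the four edge meshes.
; SetHeight then gives the main ground mesh a small biome-specific Z offset, leaving the transition meshes in place.
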(event EventOnBiomeUpdated
  (bind _grassmaterial (Variables|Default|GetGrassMaterial))
  (bind _groundtransitionmeshtop (Variables|Default|GetGroundTransitionMeshTop))
  (bind _groundtransitionmeshright (Variables|Default|GetGroundTransitionMeshRight))
  (bind _groundtransitionmeshleft (Variables|Default|GetGroundTransitionMeshLeft))
  (bind _groundmeshcomponent (Variables|Default|GetGroundMeshComponent))
  (bind _groundtransitionmeshbottom (Variables|Default|GetGroundTransitionMeshBottom))
  (bind _returnvalue (Class|MActor|GetMyBiome))
  (switch Utilities|FlowControl|Switch|SwitchonEBiome _returnvalue
    (:DarkWoods
      (|SetBy-RefVar _grassmaterial "/Game/Memoryator/Materials/3DGrass/MI_GrassSmall_DarkWoods.MI_GrassSmall_DarkWoods")
      (Rendering|Material|SetMaterial _groundmeshcomponent 0 "/Game/Memoryator/Materials/Ground/MI_DarkWoods.MI_DarkWoods")
      (Rendering|Material|SetMaterial _groundtransitionmeshbottom 0 "/Game/Memoryator/Materials/Ground/Transitions/MI_DarkWoodsTransition.MI_DarkWoodsTransition")
      (Rendering|Material|SetMaterial _groundtransitionmeshtop 0 "/Game/Memoryator/Materials/Ground/Transitions/MI_DarkWoodsTransition.MI_DarkWoodsTransition")
      (Rendering|Material|SetMaterial _groundtransitionmeshright 0 "/Game/Memoryator/Materials/Ground/Transitions/MI_DarkWoodsTransition.MI_DarkWoodsTransition")
      (Rendering|Material|SetMaterial _groundtransitionmeshleft 0 "/Game/Memoryator/Materials/Ground/Transitions/MI_DarkWoodsTransition.MI_DarkWoodsTransition")
      (CallFunction|SetHeight 0.1))
    (:BirchGrove
      (|SetBy-RefVar _grassmaterial "/Game/Memoryator/Materials/3DGrass/MI_GrassSmall_BirchGrove.MI_GrassSmall_BirchGrove")
      (Rendering|Material|SetMaterial _groundmeshcomponent 0 "/Game/Memoryator/Materials/Ground/MI_BirchGrove.MI_BirchGrove")
      (Rendering|Material|SetMaterial _groundtransitionmeshbottom 0 "/Game/Memoryator/Materials/Ground/Transitions/MI_BirchGroveTransition.MI_BirchGroveTransition")
      (Rendering|Material|SetMaterial _groundtransitionmeshtop 0 "/Game/Memoryator/Materials/Ground/Transitions/MI_BirchGroveTransition.MI_BirchGroveTransition")
      (Rendering|Material|SetMaterial _groundtransitionmeshright 0 "/Game/Memoryator/Materials/Ground/Transitions/MI_BirchGroveTransition.MI_BirchGroveTransition")
      (Rendering|Material|SetMaterial _groundtransitionmeshleft 0 "/Game/Memoryator/Materials/Ground/Transitions/MI_BirchGroveTransition.MI_BirchGroveTransition")
      (CallFunction|SetHeight 0.2))
    (:Swamp
      (|SetBy-RefVar _grassmaterial "/Game/Memoryator/Materials/3DGrass/MI_GrassSmall_Swamp.MI_GrassSmall_Swamp")
      (Rendering|Material|SetMaterial _groundmeshcomponent 0 "/Game/Memoryator/Materials/Ground/MI_SwampGround.MI_SwampGround")
      (Rendering|Material|SetMaterial _groundtransitionmeshbottom 0 "/Game/Memoryator/Materials/Ground/Transitions/MI_SwampTransition.MI_SwampTransition")
      (Rendering|Material|SetMaterial _groundtransitionmeshtop 0 "/Game/Memoryator/Materials/Ground/Transitions/MI_SwampTransition.MI_SwampTransition")
      (Rendering|Material|SetMaterial _groundtransitionmeshright 0 "/Game/Memoryator/Materials/Ground/Transitions/MI_SwampTransition.MI_SwampTransition")
      (Rendering|Material|SetMaterial _groundtransitionmeshleft 0 "/Game/Memoryator/Materials/Ground/Transitions/MI_SwampTransition.MI_SwampTransition")
      (CallFunction|SetHeight 0.0))))

(fn ConstructionScript)

(fn SetHeight
  (params (Height :type Float%20%28double-precision%29))
  (bind _groundmeshcomponent (Variables|Default|GetGroundMeshComponent))
  (bind _relativelocation (Variables|/Script/Engine.SceneComponent|GetRelativeLocation _groundmeshcomponent))
  (bind (_x _y) (Class|KismetMathLibrary|BreakVector3f _relativelocation))
  (Transformation|SetRelativeLocation _groundmeshcomponent (Math|Vector|MakeVector _x _y Height) false false))