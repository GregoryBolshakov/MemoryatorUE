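; Plant environment actor that varies its Paper2D sprite to suit the biome it is given.
; The Randomize event branches on Biome (DarkWoods, BirchGrove or Swamp) and sets SpriteTree to a random plant, mushroom or dandelion sprite from that biome's hardcoded set.
; Any other biome leaves the sprite unchanged and draws a red debug warning.
; The construction script is empty, so randomization happens only when Randomize is called.
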(event EventRandomize
  (params (Biome :type EBiome%20Enum :default "DarkWoods"))
  (bind _spritetree (Variables|Default|GetSpriteTree))
  (bind _spritetree_2 (Variables|Default|GetSpriteTree))
  (bind _spritetree_3 (Variables|Default|GetSpriteTree))
  (if (Utilities|Enum|Equal(Enum) Biome "DarkWoods")
    (switch int (Math|Random|RandomInteger 5)
      (:0
        (Rendering|Components|Sprite|SetSprite _spritetree_3 "/Game/Memoryator/Textures/Environment/DarkWoods/Frames/DarkWoods_plant_8_png.DarkWoods_plant_8_png"))
      (:1
        (Rendering|Components|Sprite|SetSprite _spritetree_3 "/Game/Memoryator/Textures/Environment/DarkWoods/Frames/DarkWoods_plant_6_png.DarkWoods_plant_6_png"))
      (:2
        (Rendering|Components|Sprite|SetSprite _spritetree_3 "/Game/Memoryator/Textures/Environment/DarkWoods/Frames/DarkWoods_plant_7_png.DarkWoods_plant_7_png"))
      (:3
        (Rendering|Components|Sprite|SetSprite _spritetree_3 "/Game/Memoryator/Textures/Environment/DarkWoods/Frames/DarkWoods_plant_8_png.DarkWoods_plant_8_png"))
      (:4
        (Rendering|Components|Sprite|SetSprite _spritetree_3 "/Game/Memoryator/Textures/Environment/DarkWoods/Frames/DarkWoods_plant_9_png.DarkWoods_plant_9_png")))
    (elif (Utilities|Enum|Equal(Enum) Biome "BirchGrove")
      (switch int (Math|Random|RandomInteger 6)
        (:0
          (Rendering|Components|Sprite|SetSprite _spritetree_2 "/Game/Memoryator/Textures/Environment/BirchGrove/Frames/mushroom_1_png.mushroom_1_png"))
        (:1
          (Rendering|Components|Sprite|SetSprite _spritetree_2 "/Game/Memoryator/Textures/Environment/BirchGrove/Frames/mushroom_2_png.mushroom_2_png"))
        (:2
          (Rendering|Components|Sprite|SetSprite _spritetree_2 "/Game/Memoryator/Textures/Environment/BirchGrove/Frames/plant_2_png.plant_2_png"))
        (:3
          (Rendering|Components|Sprite|SetSprite _spritetree_2 "/Game/Memoryator/Textures/Environment/BirchGrove/Frames/plant_7_png.plant_7_png"))
        (:4
          (Rendering|Components|Sprite|SetSprite _spritetree_2 "/Game/Memoryator/Textures/Environment/BirchGrove/Frames/plant_6_png.plant_6_png"))
        (:5
          (Rendering|Components|Sprite|SetSprite _spritetree_2 "/Game/Memoryator/Textures/Environment/BirchGrove/Frames/plant_8_png.plant_8_png")))
      (elif (Utilities|Enum|Equal(Enum) Biome "Swamp")
        (switch int (Math|Random|RandomInteger 8)
          (:0
            (Rendering|Components|Sprite|SetSprite _spritetree "/Game/Memoryator/Textures/Environment/Swamp/Frames/SwampyTrees_dandelion_1_png.SwampyTrees_dandelion_1_png"))
          (:1
            (Rendering|Components|Sprite|SetSprite _spritetree "/Game/Memoryator/Textures/Environment/Swamp/Frames/SwampyTrees_dandelion_2_png.SwampyTrees_dandelion_2_png"))
          (:2
            (Rendering|Components|Sprite|SetSprite _spritetree "/Game/Memoryator/Textures/Environment/Swamp/Frames/SwampyTrees_dandelion_3_png.SwampyTrees_dandelion_3_png"))
          (:3
            (Rendering|Components|Sprite|SetSprite _spritetree "/Game/Memoryator/Textures/Environment/Swamp/Frames/SwampyTrees_mushroom_1_png.SwampyTrees_mushroom_1_png"))
          (:4
            (Rendering|Components|Sprite|SetSprite _spritetree "/Game/Memoryator/Textures/Environment/Swamp/Frames/SwampyTrees_mushroom_2_png.SwampyTrees_mushroom_2_png"))
          (:5
            (Rendering|Components|Sprite|SetSprite _spritetree "/Game/Memoryator/Textures/Environment/Swamp/Frames/SwampyTrees_mushroom_3_png.SwampyTrees_mushroom_3_png"))
          (:6
            (Rendering|Components|Sprite|SetSprite _spritetree "/Game/Memoryator/Textures/Environment/Swamp/Frames/SwampyTrees_mushroom_4_png.SwampyTrees_mushroom_4_png"))
          (:7
            (Rendering|Components|Sprite|SetSprite _spritetree "/Game/Memoryator/Textures/Environment/Swamp/Frames/SwampyTrees_plant_3_png.SwampyTrees_plant_3_png")))
        (else
          (Rendering|Debug|DrawDebugString "0, 0, 0" "No biome specified" 0 "(R=1.000000,G=0.000000,B=0.000000,A=1.000000)" 5.0))))))

(fn ConstructionScript)