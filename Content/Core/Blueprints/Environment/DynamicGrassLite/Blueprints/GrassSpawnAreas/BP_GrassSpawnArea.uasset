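; Grass spawn area actor that defines a volume for the Dynamic Grass Lite system to fill with biome-specific grass.
; Construction picks a random geometry preset from a data asset and builds translucent procedural floor and ceiling meshes, with instanced pillars visualizing height.
; On BeginPlay or OnEnabled, it swaps the grass mesh to match its biome and asks the foliage manager to spawn once.
; A name-check workaround skips "TestBounds_" instances.
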(event EventBeginPlay
  (bind _foliagetospawn (Variables|Default|GetfoliageToSpawn))
  (bind _foliagetospawn_2 (Variables|Default|GetfoliageToSpawn))
  (bind _output (Utilities|Array|Get(acopy) _foliagetospawn))
  ;[1 1 1] TODO: get rid of this workaround
  (if (not (Utilities|String|Contains (Utilities|GetObjectName self) "TestBounds_"))
    (if (not (Variables|Default|GetIsCreated))
      (Variables|Default|SetIsCreated true)
      ;[1 1 1 1 26] Set biome (TODO: Make it more beautiful)
      (bind _returnvalue (Class|MActor|GetMyBiome))
      (switch Utilities|FlowControl|Switch|SwitchonEBiome _returnvalue
        (:DarkWoods
          (Utilities|Array|SetArrayElem _foliagetospawn_2 0 (Utilities|Struct|MakeFoliageToSpawnInArea "/Game/Core/Environment/Vegetation/Grass/Meshes/SM_Grass_SmallGroup_DarkWoods.SM_Grass_SmallGroup_DarkWoods" (.foliagetospawn_component _output) (.density _output) (.irregularity _output) (.minscale _output) (.maxscale _output))))
        (:BirchGrove
          (Utilities|Array|SetArrayElem _foliagetospawn_2 0 (Utilities|Struct|MakeFoliageToSpawnInArea "/Game/Core/Environment/Vegetation/Grass/Meshes/SM_Grass_SmallGroup_BirchGrove.SM_Grass_SmallGroup_BirchGrove" (.foliagetospawn_component _output) (.density _output) (.irregularity _output) (.minscale _output) (.maxscale _output))))
        (:Swamp
          (Utilities|Array|SetArrayElem _foliagetospawn_2 0 (Utilities|Struct|MakeFoliageToSpawnInArea "/Game/Core/Environment/Vegetation/Grass/Meshes/SM_Grass_SmallGroup_Swamp.SM_Grass_SmallGroup_Swamp" (.foliagetospawn_component _output) (.density _output) (.irregularity _output) (.minscale _output) (.maxscale _output)))))
      (Default|SpawnGrassinArea (Variables|/Game/Core/Blueprints/Environment/DynamicGrassLite/Blueprints/InternalLogic/INTERACTIVE_FoliageComp_BP.INTERACTIVE_FoliageComp_BP_C|GetManager (Variables|Default|GetFoliage%20Component)) self))))

(event EventOnEnabled
  (bind _foliagetospawn (Variables|Default|GetfoliageToSpawn))
  (bind _foliagetospawn_2 (Variables|Default|GetfoliageToSpawn))
  (bind _output (Utilities|Array|Get(acopy) _foliagetospawn))
  ;[1 1 1] TODO: get rid of this workaround
  (if (not (Utilities|String|Contains (Utilities|GetObjectName self) "TestBounds_"))
    (if (not (Variables|Default|GetIsCreated))
      (Variables|Default|SetIsCreated true)
      ;[1 1 1 1 26] Set biome (TODO: Make it more beautiful)
      (bind _returnvalue (Class|MActor|GetMyBiome))
      (switch Utilities|FlowControl|Switch|SwitchonEBiome _returnvalue
        (:DarkWoods
          (Utilities|Array|SetArrayElem _foliagetospawn_2 0 (Utilities|Struct|MakeFoliageToSpawnInArea "/Game/Core/Environment/Vegetation/Grass/Meshes/SM_Grass_SmallGroup_DarkWoods.SM_Grass_SmallGroup_DarkWoods" (.foliagetospawn_component _output) (.density _output) (.irregularity _output) (.minscale _output) (.maxscale _output))))
        (:BirchGrove
          (Utilities|Array|SetArrayElem _foliagetospawn_2 0 (Utilities|Struct|MakeFoliageToSpawnInArea "/Game/Core/Environment/Vegetation/Grass/Meshes/SM_Grass_SmallGroup_BirchGrove.SM_Grass_SmallGroup_BirchGrove" (.foliagetospawn_component _output) (.density _output) (.irregularity _output) (.minscale _output) (.maxscale _output))))
        (:Swamp
          (Utilities|Array|SetArrayElem _foliagetospawn_2 0 (Utilities|Struct|MakeFoliageToSpawnInArea "/Game/Core/Environment/Vegetation/Grass/Meshes/SM_Grass_SmallGroup_Swamp.SM_Grass_SmallGroup_Swamp" (.foliagetospawn_component _output) (.density _output) (.irregularity _output) (.minscale _output) (.maxscale _output)))))
      (Default|SpawnGrassinArea (Variables|/Game/Core/Blueprints/Environment/DynamicGrassLite/Blueprints/InternalLogic/INTERACTIVE_FoliageComp_BP.INTERACTIVE_FoliageComp_BP_C|GetManager (Variables|Default|GetFoliage%20Component)) self))))

(fn ConstructionScript
  (bind _proceduralmesh (Variables|Default|GetProceduralMesh))
  (bind _proceduralmesh_2 (Variables|Default|GetProceduralMesh))
  ;[1 1 1] Get random geometry preset
  (bind _output_get (Variables|Default|SetGeometryPreset (.OutItem (Utilities|Array|Random (Variables|/Script/TopDownTemp.GrassSpawnAreaGeometryDataAsset|GetPresets (Variables|Default|GetGeometryDataAsset))))))
  (Variables|Default|SetV (.v _output_get))
  (Variables|Default|Settriangles (.triangles _output_get))
  (Variables|Default|SetareaHeight (.areaheight _output_get))
  (Variables|Default|SetV_Ceiling (.v_celling _output_get))
  (if true
    (Class|ProceduralMeshComponent|CreateMeshSectionLinearColor _proceduralmesh_2 0 (Variables|Default|GetV) (Variables|Default|Gettriangles) 0 0 0 0 0 0 0 true false)
    (Rendering|Material|SetMaterial _proceduralmesh_2 0 "/Game/Core/Blueprints/Environment/DynamicGrassLite/Materials/Misc/SimpleTranslucent_M.SimpleTranslucent_M")
    (Components|InstancedStaticMesh|ClearInstances (Variables|Default|GetHeightVisPillars))
    (Utilities|Array|Clear (Variables|Default|GetV_Ceiling))
    (for _array_element (Variables|Default|GetV)
      (Utilities|Array|Add (Variables|Default|GetV_Ceiling) (+ _array_element (Math|Vector|MakeVector 0.0 0.0 (Variables|Default|GetareaHeight))))
      (Components|InstancedStaticMesh|AddInstance (Variables|Default|GetHeightVisPillars) (Math|Transform|MakeTransform _array_element "0, 0, 0" (Math|Vector|MakeVector 0.01 0.01 (Variables|Default|GetareaHeight))) false))
    (Class|ProceduralMeshComponent|CreateMeshSectionLinearColor _proceduralmesh 1 (Variables|Default|GetV_Ceiling) (Variables|Default|Gettriangles) 0 0 0 0 0 0 0 false false)
    (Rendering|Material|SetMaterial _proceduralmesh 1 "/Game/Core/Blueprints/Environment/DynamicGrassLite/Materials/Misc/SimpleTranslucent_M.SimpleTranslucent_M")
    (else
      (Utilities|String|LogString "Couldn't find geometry preset"))))