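; Yarrow flower environment object, a pickable sprite item that holds a small random amount of a single item type.
; On BeginPlay it initialises its inventory with that item in a randomised quantity.
; Its Randomize event sets the pickable sprite to one of several yarrow variants chosen at random, varying the plant's look.
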(event EventRandomize
  (params (Biome :type EBiome%20Enum :default "DarkWoods"))
  (bind _spritepickableiem (Variables|Default|GetSpritePickableIem))
  (switch int (Math|Random|RandomInteger 5)
    (:0
      (Rendering|Components|Sprite|SetSprite _spritepickableiem "/Game/Core/Environment/Vegetation/2DFlowers/Sprites/flowers_yarrow_1_png.flowers_yarrow_1_png"))
    (:1
      (Rendering|Components|Sprite|SetSprite _spritepickableiem "/Game/Core/Environment/Vegetation/2DFlowers/Sprites/flowers_yarrow_2_png.flowers_yarrow_2_png"))
    (:2
      (Rendering|Components|Sprite|SetSprite _spritepickableiem "/Game/Core/Environment/Vegetation/2DFlowers/Sprites/flowers_yarrow_3_png.flowers_yarrow_3_png"))
    (:3
      (Rendering|Components|Sprite|SetSprite _spritepickableiem "/Game/Core/Environment/Vegetation/2DFlowers/Sprites/flowers_yarrow_4_png.flowers_yarrow_4_png"))
    (:4
      (Rendering|Components|Sprite|SetSprite _spritepickableiem "/Game/Core/Environment/Vegetation/2DFlowers/Sprites/flowers_yarrow_5_png.flowers_yarrow_5_png"))))

(event EventBeginPlay
  (Class|MPickableActor|InitialiseInventory (Utilities|Array|MakeArray (Utilities|Struct|MakeItem 5 (Math|Random|RandomIntegerinRange 1 3)))))

(fn ConstructionScript)