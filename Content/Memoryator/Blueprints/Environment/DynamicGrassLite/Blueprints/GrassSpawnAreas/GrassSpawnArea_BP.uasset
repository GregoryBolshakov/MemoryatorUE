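; Grass spawn area actor that defines a region for the foliage manager to fill with grass.
; Construction picks a random geometry preset and builds a translucent procedural floor with collision, a ceiling copy raised by area height, and instanced pillars visualizing that height.
; On BeginPlay or OnEnabled it requests grass once from the manager, skipping objects named "TestBounds_" as a marked workaround.
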(event EventBeginPlay
  ;[1 1 1] TODO: get rid of this workaround
  (if (not (Utilities|String|Contains (Utilities|GetObjectName self) "TestBounds_"))
    (if (not (Variables|Default|GetIsCreated))
      (Variables|Default|SetIsCreated true)
      (Default|SpawnGrassinArea (Variables|/Game/Memoryator/Blueprints/Environment/DynamicGrassLite/Blueprints/InternalLogic/INTERACTIVE_FoliageComp_BP.INTERACTIVE_FoliageComp_BP_C|GetManager (Variables|Default|GetFoliage%20Component)) self))))

(event EventOnEnabled
  ;[1 1 1] TODO: get rid of this workaround
  (if (not (Utilities|String|Contains (Utilities|GetObjectName self) "TestBounds_"))
    (if (not (Variables|Default|GetIsCreated))
      (Variables|Default|SetIsCreated true)
      (Default|SpawnGrassinArea (Variables|/Game/Memoryator/Blueprints/Environment/DynamicGrassLite/Blueprints/InternalLogic/INTERACTIVE_FoliageComp_BP.INTERACTIVE_FoliageComp_BP_C|GetManager (Variables|Default|GetFoliage%20Component)) self))))

(fn ConstructionScript
  (bind _proceduralmesh (Variables|Default|GetProceduralMesh))
  (bind _proceduralmesh_2 (Variables|Default|GetProceduralMesh))
  ;[1 1 1] Get random geometry preset
  (bind _output_get (Variables|Default|SetNewVar (.OutItem (Utilities|Array|Random (Variables|/Script/TopDownTemp.GrassSpawnAreaGeometryDataAsset|GetPresets (Variables|Default|GetGeometryDataAsset))))))
  (Variables|Default|SetV (.v _output_get))
  (Variables|Default|Settriangles (.triangles _output_get))
  (Variables|Default|SetareaHeight (.areaheight _output_get))
  (Variables|Default|SetV_Ceiling (.v_celling _output_get))
  (if true
    (Class|ProceduralMeshComponent|CreateMeshSectionLinearColor _proceduralmesh_2 0 (Variables|Default|GetV) (Variables|Default|Gettriangles) 0 0 0 0 0 0 0 true false)
    (Rendering|Material|SetMaterial _proceduralmesh_2 0 "/Game/Memoryator/Blueprints/Environment/DynamicGrassLite/Materials/Misc/SimpleTranslucent_M.SimpleTranslucent_M")
    (Components|InstancedStaticMesh|ClearInstances (Variables|Default|GetHeightVisPillars))
    (Utilities|Array|Clear (Variables|Default|GetV_Ceiling))
    (for _array_element (Variables|Default|GetV)
      (Utilities|Array|Add (Variables|Default|GetV_Ceiling) (+ _array_element (Math|Vector|MakeVector 0.0 0.0 (Variables|Default|GetareaHeight))))
      (Components|InstancedStaticMesh|AddInstance (Variables|Default|GetHeightVisPillars) (Math|Transform|MakeTransform _array_element "0, 0, 0" (Math|Vector|MakeVector 0.01 0.01 (Variables|Default|GetareaHeight))) false))
    (Class|ProceduralMeshComponent|CreateMeshSectionLinearColor _proceduralmesh 1 (Variables|Default|GetV_Ceiling) (Variables|Default|Gettriangles) 0 0 0 0 0 0 0 false false)
    (Rendering|Material|SetMaterial _proceduralmesh 1 "/Game/Memoryator/Blueprints/Environment/DynamicGrassLite/Materials/Misc/SimpleTranslucent_M.SimpleTranslucent_M")
    (else
      (Utilities|String|LogString "Couldn't find geometry preset"))))