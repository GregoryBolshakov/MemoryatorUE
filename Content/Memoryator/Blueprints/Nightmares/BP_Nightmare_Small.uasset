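; Small nightmare mob Blueprint that drives its flipbook body animation from combat and movement state.
; UpdateAnimation clears old delegates, then picks TakeDamage, Move, Fight or Idle in that priority order.
; Fight binds animation completion and notifies the MMobController cached on possession when a specific striking frame plays.
; When the damage animation ends, it resets the color and damage flag, sets idle behavior through the controller and refreshes the animation.
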(event Custom|CustomEvent_0
  (bind _self self)
  ;[1 1 1] Take damage animation
  (Class|M2DRepresentationComponent|SetColor (Variables|Default|GetRepresentationComponent) (Class|KismetMathLibrary|LinearColorWhite))
  (Variables|Default|SetIsTakingDamage false)
  (bind _returnvalue (Class|TypedElementWorldInterface|GetOwnerWorld(Message) _self (Utilities|Struct|MakeScriptTypedElementHandle)))
  (Class|MInterfaceMobController|SetIdleBehavior (Variables|Default|GetMobController) _returnvalue _self)
  (Class|MCharacter|UpdateAnimation))

(event Custom|OnSpriteChanged
  ;[1 1 1] Fight animation
  ;;[1 1 1] Bind the striking sprite of the animation with controller
  (if (== (Class|PaperFlipbookComponent|GetPlaybackPositioninFrames (Variables|Default|GetFlipbookBody)) 5)
    (Class|MMobController|OnHit (Variables|Default|GetMobController))))

(event EventUpdateAnimation
  (bind _flipbookbody (Variables|Default|GetFlipbookBody))
  (bind _flipbookbody_2 (Variables|Default|GetFlipbookBody))
  ;[1 1 1] Reset all bindings and play flipbook from start
  (EventDispatchers|UnbindallEventsfromOnFinishedPlaying _flipbookbody)
  (EventDispatchers|UnbindallEventsfromOnSpriteChangeDelegate _flipbookbody)
  (Components|Timeline|PlayfromStart _flipbookbody)
  (if (Variables|Default|GetIsTakingDamage)
    ;[1 1 1] Take damage animation
    (Class|MRotatableFlipbookComponent|SetAction _flipbookbody_2 (Utilities|Name|MakeLiteralName "TakeDamage"))
    (EventDispatchers|BindEventtoOnFinishedPlaying _flipbookbody_2 (delegate Custom|CustomEvent_0))
    (elif (Variables|Default|GetIsMoving)
      ;[1 1 1] Move animation
      (Class|MRotatableFlipbookComponent|SetAction (Variables|Default|GetFlipbookBody) (Utilities|Name|MakeLiteralName "Move"))
      (elif (Variables|Default|GetIsFighting)
        ;[1 1 1] Fight animation
        (Class|MRotatableFlipbookComponent|SetAction (Variables|Default|GetFlipbookBody) (Utilities|Name|MakeLiteralName "Fight"))
        ;;[1 1 1] Bind the end of the fight animation with controller
        (EventDispatchers|BindEventtoOnFinishedPlaying (Variables|Default|GetFlipbookBody) (EventDispatchers|CreateEvent (Variables|Default|GetMobController) :!event OnFightAnimationEnd))
        ;;[1 1 1] Bind the striking sprite of the animation with controller
        (EventDispatchers|BindEventtoOnSpriteChangeDelegate (Variables|Default|GetFlipbookBody) (delegate Custom|OnSpriteChanged))
        (else
          ;[1 1 1] Idle animation
          (Class|MRotatableFlipbookComponent|SetAction (Variables|Default|GetFlipbookBody) (Utilities|Name|MakeLiteralName "Idle")))))))

(event EventPossessed
  (params (NewController :type Controller%20Object%20Reference))
  (bind _asmmob_controller (Utilities|Casting|CastToMMobController (Pawn|GetController)))
  (Variables|Default|SetMobController _asmmob_controller))

(fn ConstructionScript)