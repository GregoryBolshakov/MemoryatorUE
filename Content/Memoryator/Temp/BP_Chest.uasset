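; Chest Blueprint that shows a circular progress bar when its Box trigger is overlapped, with no opening or reward logic.
; BeginPlay casts the Widget component's user widget to WBP_CircularProgressBar and caches it.
; Any begin overlap restarts a timeline that feeds the bar's progress on each update.
; End overlap sets progress to zero but does not stop the timeline, so a running timeline keeps updating the bar.
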(event OnComponentBeginOverlap(Box)
  (params (OverlappedComponent :type Primitive%20Component%20Object%20Reference) (OtherActor :type Actor%20Object%20Reference) (OtherComp :type Primitive%20Component%20Object%20Reference) (OtherBodyIndex :type Integer) (bFromSweep :type Boolean) (SweepResult :type Hit%20Result%20Structure%20%28by%20ref%29))
  (bind _0_1 (Timeline|Timeline_0 PlayFromStart)
    (:Update
      (Default|SetProgress (Variables|Default|GetProgressWidget) _0_1))))

(event OnComponentEndOverlap(Box)
  (params (OverlappedComponent :type Primitive%20Component%20Object%20Reference) (OtherActor :type Actor%20Object%20Reference) (OtherComp :type Primitive%20Component%20Object%20Reference) (OtherBodyIndex :type Integer))
  (Default|SetProgress (Variables|Default|GetProgressWidget) 0.0))

(event EventBeginPlay
  (bind _ascircular_progress_bar_widget (Utilities|Casting|CastToWBP_CircularProgressBar (UserInterface|GetUserWidgetObject (Variables|Default|GetWidget))))
  (Variables|Default|SetProgressWidget _ascircular_progress_bar_widget))

(fn ConstructionScript)