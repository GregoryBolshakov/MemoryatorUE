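; BP_Memoryator is the player-possessed 2.5D character, driving separate body and legs flipbooks from its damage, dash, fight, move and idle states.
; UpdateAnimation rebinds delegates and restarts only flipbooks whose action changed; attacks activate Niagara and trigger the controller's hit on a specific body frame.
; Reverse movement plays legs backwards, stops sprint and tilts the sprite by camera angle.
; Tick writes the actor's location to the MPC_Walls material parameter collection.
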(event Custom|CustomEvent_0
  ;[1 1 1] Take damage animation
  (Class|M2DRepresentationComponent|SetColor (Variables|Default|GetRepresentationComponent) (Class|KismetMathLibrary|LinearColorWhite))
  (Variables|Default|SetIsTakingDamage false)
  (Class|MCharacter|UpdateAnimation))

(event Custom|OnReverseMovementStarted
  (bind _representationcomponent (Variables|Default|GetRepresentationComponent))
  ;[1 1 1 1 32] Reverse move design
  (Utilities|String|Reverse (Variables|Default|GetFlipbookLegs))
  (Class|MPlayerController|TurnSprintOff (Variables|Default|GetMPlayerController))
  (bind _returnvalue (Class|M2DRepresentationBlueprintLibrary|GetCameraDeflectionAngle self (Transformation|GetVelocity)))
  (if (and (>= _returnvalue 45.0) (<= _returnvalue 135.0))
    (Variables|/Script/TopDownTemp.M2DRepresentationComponent|SetRotationWhileFacingCamera _representationcomponent "-6.000000, 0, 0")
    (elif (and (<= _returnvalue -45.0) (>= _returnvalue -135.0))
      (Variables|/Script/TopDownTemp.M2DRepresentationComponent|SetRotationWhileFacingCamera _representationcomponent "6.000000, 0, 0")
      (else
        (Variables|/Script/TopDownTemp.M2DRepresentationComponent|SetRotationWhileFacingCamera _representationcomponent "0, 0, 0")))))

(event Custom|On%20Sprite%20Changed
  ;[1 1 1] Fight animation
  (if (== (Class|PaperFlipbookComponent|GetPlaybackPositioninFrames (Variables|Default|GetFlipbookBody)) 5)
    (Class|MPlayerController|OnHit (Variables|Default|GetMPlayerController))))

(event Custom|OnReverseMovementStopped
  ;[1 1 1 1 32] Reverse move design
  (Audio|Components|Audio|Play (Variables|Default|GetFlipbookLegs))
  (Variables|/Script/TopDownTemp.M2DRepresentationComponent|SetRotationWhileFacingCamera (Variables|Default|GetRepresentationComponent) "0, 0, 0"))

(event Custom|On%20Attack%20End
  ;[1 1 1] Fight animation
  (Class|MCharacter|SetIsFighting false))

(event EventTick
  (params (DeltaSeconds :type Float%20%28single-precision%29))
  (Rendering|Material|SetVectorParameterValue "/Game/EpicGamesAssets/Wall_Hiding_System/Materials/Material_Functions/MPC_Walls.MPC_Walls" "Location_1" (Math|Conversions|ToLinearColor(Vector) (Transformation|GetActorLocation)) :!class /Script/Engine.KismetMaterialLibrary))

(event EventUpdateAnimation
  (bind _flipbookbody (Variables|Default|GetFlipbookBody))
  (bind _flipbookbody_2 (Variables|Default|GetFlipbookBody))
  (bind _flipbookbody_3 (Variables|Default|GetFlipbookBody))
  (bind _flipbooklegs (Variables|Default|GetFlipbookLegs))
  ;[1 1 1 1 32] Reset all bindings and play flipbook from start
  (Utilities|FlowControl|Sequence
    (:then_0
      (EventDispatchers|UnbindallEventsfromOnReverseMovementStartedDelegate))
    (:then_1
      (EventDispatchers|UnbindallEventsfromOnFinishedPlaying _flipbookbody_2)
      (EventDispatchers|UnbindallEventsfromOnSpriteChangeDelegate _flipbookbody_2))
    (:then_2
      (Components|Activation|Deactivate (Variables|Default|GetNiagara)))
    (:then_3
      (Variables|Default|SetLastLegsAction (Class|MRotatableFlipbookComponent|GetAction (Variables|Default|GetFlipbookLegs)))
      (Variables|Default|SetLastBodyAction (Class|MRotatableFlipbookComponent|GetAction (Variables|Default|GetFlipbookBody)))
      (if (Variables|Default|GetIsMoving)
        ;[1 1 1 1 32] Reverse move design
        (EventDispatchers|BindEventtoOnReverseMovementStartedDelegate (delegate Custom|OnReverseMovementStarted))
        (EventDispatchers|BindEventtoOnReverseMovementStoppedDelegate (delegate Custom|OnReverseMovementStopped)))
      (if (Variables|Default|GetIsTakingDamage)
        ;[1 1 1] Take damage animation
        (Class|MRotatableFlipbookComponent|SetAction (Variables|Default|GetFlipbookLegs) (Utilities|Name|MakeLiteralName "None"))
        (Class|MRotatableFlipbookComponent|SetAction _flipbookbody (Utilities|Name|MakeLiteralName "TakeDamage"))
        (EventDispatchers|BindEventtoOnFinishedPlaying _flipbookbody (delegate Custom|CustomEvent_0))
        (elif (Variables|Default|GetIsDashing)
          ;[1 1 1] Dash animation
          (Class|MRotatableFlipbookComponent|SetAction (Variables|Default|GetFlipbookBody) (Utilities|Name|MakeLiteralName "Dash"))
          (Class|MRotatableFlipbookComponent|SetAction (Variables|Default|GetFlipbookLegs) (Utilities|Name|MakeLiteralName "Dash"))
          (elif (Variables|Default|GetIsFighting)
            ;[1 1 1] Fight animation
            (Class|MRotatableFlipbookComponent|SetAction (Variables|Default|GetFlipbookBody) (Utilities|Name|MakeLiteralName "Fight"))
            (if (Variables|Default|GetIsMoving)
              (Class|MRotatableFlipbookComponent|SetAction (Variables|Default|GetFlipbookLegs) (Utilities|Name|MakeLiteralName "Move"))
              (else
                (Class|MRotatableFlipbookComponent|SetAction (Variables|Default|GetFlipbookLegs) (Utilities|Name|MakeLiteralName "Fight"))))
            (Components|Activation|Activate (Variables|Default|GetNiagara) false)
            (EventDispatchers|BindEventtoOnFinishedPlaying (Variables|Default|GetFlipbookBody) (delegate Custom|On%20Attack%20End))
            (EventDispatchers|BindEventtoOnSpriteChangeDelegate (Variables|Default|GetFlipbookBody) (delegate Custom|On%20Sprite%20Changed))
            (elif (Variables|Default|GetIsMoving)
              ;[1 1 1] Move animation
              (Class|MRotatableFlipbookComponent|SetAction (Variables|Default|GetFlipbookBody) (Utilities|Name|MakeLiteralName "Move"))
              (Class|MRotatableFlipbookComponent|SetAction (Variables|Default|GetFlipbookLegs) (Utilities|Name|MakeLiteralName "Move"))
              (else
                ;[1 1 1] Idle animation
                (Class|MRotatableFlipbookComponent|SetAction (Variables|Default|GetFlipbookBody) (Utilities|Name|MakeLiteralName "Idle"))
                (Class|MRotatableFlipbookComponent|SetAction (Variables|Default|GetFlipbookLegs) (Utilities|Name|MakeLiteralName "Idle"))))))))
    (:then_4
      ;[1 1 1] Play flipbook from start only if the action was changed
      (if (!= (Class|MRotatableFlipbookComponent|GetAction _flipbooklegs) (Variables|Default|GetLastLegsAction))
        (Components|Timeline|PlayfromStart _flipbooklegs))
      (if (!= (Class|MRotatableFlipbookComponent|GetAction _flipbookbody_3) (Variables|Default|GetLastBodyAction))
        (Components|Timeline|PlayfromStart _flipbookbody_3)))))

(event EventPossessed
  (params (NewController :type Controller%20Object%20Reference))
  (bind _asmplayer_controller (Utilities|Casting|CastToMPlayerController (Pawn|GetController)))
  (Variables|Default|SetMPlayerController _asmplayer_controller))

(fn ConstructionScript)